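; Base factory actor with optional input and output slot child actors and an output item stack.
; The Construction Script caches each enabled BP_BaseIOSlot and registers the factory as its parent, destroying disabled or invalid slot actors and clearing their flags.
; InternalGrabItemOutput removes one item from the output stack and returns its type, or fails when empty.
; The power check is an empty stub, and EventGraph holds an unused copy of the slot setup.
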(event EventBeginPlay)

(fn ConstructionScript
  (Utilities|FlowControl|Sequence
    (:then_0
      ;[1 1 1] Setup Input
      (if (Variables|Default|GetHasInput?)
        (bind _asbp_base_ioslot (Utilities|Casting|CastToBP_BaseIOSlot (Variables|/Script/Engine.ChildActorComponent|GetChildActor (Variables|Default|GetInput)))
          (:then
            (bind _output_get (Variables|Default|SetInputSlot _asbp_base_ioslot))
            (Class|InteractionInterface|RegisterSlotParent(Message) _output_get self))
          (:CastFailed
            (Variables|Default|SetHasInput? false :!label _label)
            (Actor|DestroyActor (Variables|/Script/Engine.ChildActorComponent|GetChildActor (Variables|Default|GetInput)))))
        (else
          (goto _label))))
    (:then_1
      ;[1 1 1] Setup Output
      (if (Variables|Default|GetHasOutput?)
        (bind _asbp_base_ioslot_2 (Utilities|Casting|CastToBP_BaseIOSlot (Variables|/Script/Engine.ChildActorComponent|GetChildActor (Variables|Default|GetOutput)))
          (:then
            (bind _output_get_2 (Variables|Default|SetOutputSlot _asbp_base_ioslot_2))
            (Class|InteractionInterface|RegisterSlotParent(Message) _output_get_2 self))
          (:CastFailed
            (Variables|Default|SetHasOutput? false :!label _label_2)
            (Actor|DestroyActor (Variables|/Script/Engine.ChildActorComponent|GetChildActor (Variables|Default|GetOutput)))))
        (else
          (goto _label_2))))
    (:then_2
      (if (Variables|Default|GetRequiresPower?)
        _))))

(fn InternalGrabItemOutput
  (bind _outputitemslot (Variables|Default|GetOutputItemSlot))
  (if (> (.CurrentStackSize (Utilities|Struct|BreakS_ItemSlot (Variables|Default|GetOutputItemSlot))) 0)
    (bind _structout (Utilities|Struct|SetmembersinS_ItemSlot _outputitemslot (- (.CurrentStackSize (Utilities|Struct|BreakS_ItemSlot _outputitemslot)) 1)))
    (return true (.itemtypeenum (.Item (Utilities|Struct|BreakS_ItemSlot _structout))))
    (else
      (return false "NewEnumerator0"))))