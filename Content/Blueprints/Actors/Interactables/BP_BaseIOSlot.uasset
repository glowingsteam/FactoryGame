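; Base input/output slot for factory interactables, giving an attach point and a way to pull items from the owning parent.
; The construction script builds a box, sphere or capsule collision component from CollisionType and CollisionSize, and moves the Billboard to the attach offset.
; A registered Parent handles item grabs, while factory queries return slot status and Billboard location.
; Miner and resource node functions return stub values.
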(event EventRegisterSlotParent
  (params (Parent :type BP%20Base%20IO%20Factory%20Object%20Reference))
  (Variables|Default|SetParent Parent))

(fn ConstructionScript
  (bind _defaultsceneroot (Variables|Default|GetDefaultSceneRoot))
  (bind _collisionsize (Variables|Public|GetCollisionSize))
  (bind _returnvalue (Transformation|GetWorldTransform _defaultsceneroot))
  (Utilities|FlowControl|Sequence
    (:then_0
      (switch Utilities|FlowControl|Switch|SwitchonE_SlotCollisionType (Variables|Public|GetCollisionType)
        (:NewEnumerator0
          (bind _returnvalue_2 (AddComponent|AddBoxComponent false _returnvalue))
          (bind _output_get (Variables|Default|SetCollisionComponent _returnvalue_2))
          (bind _asbox_collision (Utilities|Casting|CastToBoxComponent _output_get))
          (Components|Box|SetBoxExtent _asbox_collision (Variables|Public|GetCollisionSize) true)
          (Collision|SetCollisionProfileName _asbox_collision "None" true :!class /Script/Engine.PrimitiveComponent))
        (:NewEnumerator1
          (bind _returnvalue_3 (AddComponent|AddSphereComponent false _returnvalue))
          (bind _output_get_2 (Variables|Default|SetCollisionComponent _returnvalue_3))
          (bind _assphere_collision (Utilities|Casting|CastToSphereComponent _output_get_2))
          (Components|Sphere|SetSphereRadius _assphere_collision (.x (Variables|Public|GetCollisionSize)) true)
          (Collision|SetCollisionProfileName _assphere_collision "None" true :!class /Script/Engine.PrimitiveComponent))
        (:NewEnumerator2
          (bind _returnvalue_4 (AddComponent|AddCapsuleComponent false _returnvalue))
          (bind _output_get_3 (Variables|Default|SetCollisionComponent _returnvalue_4))
          (bind _ascapsule_collision (Utilities|Casting|CastToCapsuleComponent _output_get_3))
          (Components|Capsule|SetCapsuleRadius _ascapsule_collision (.x _collisionsize) true)
          (Components|Capsule|SetCapsuleHalfHeight _ascapsule_collision (.y _collisionsize) true)
          (Collision|SetCollisionProfileName _ascapsule_collision "None" true :!class /Script/Engine.PrimitiveComponent)))
      (Transformation|SetWorldLocation (Variables|Default|GetCollisionComponent) (Transformation|GetWorldLocation (Variables|Default|GetDefaultSceneRoot)) false true))
    (:then_1
      (Transformation|SetRelativeLocation (Variables|Default|GetBillboard) (Variables|Public|GetAttachPointOffset) false true))))

(fn AttachMiner
  (return "0, 0, 0" "NewEnumerator0"))

(fn GrabItemfromOutput
  (bind _parent (Variables|Default|GetParent))
  (Utilities|IsValid _parent
    (:Is%20Valid
      (bind (_success_ _itempulled) (Class|FactoryInternalInterface|InternalGrabItemOutput(Message) _parent))
      (return _success_ _itempulled))
    (:Is%20Not%20Valid
      (Development|PrintString "Parent Not Valid")
      (return false "NewEnumerator0"))))

(fn QueryFactory
  (return true (Variables|Public|GetFactoryStatus) (Transformation|GetWorldLocation (Variables|Default|GetBillboard)) false))

(fn QueryResourceNode
  (return false false "NewEnumerator0"))