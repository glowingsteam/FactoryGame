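; Item tube actor that runs a spline-mesh pipe between two IO slots and visually carries items along it.
; A looping timer shifts items through spacing-sized array slots, pulls new ones from the input slot and removes those at the far end without passing them on.
; Items render as HISM instances, pooled per model and material, with parallel arrays tracking each slot's component and instance index.
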(event Custom|ProcessItems
  (CallFunction|PushItemsThroughArray))

(event EventBeginPlay
  (if (and (Utilities|IsValid (Variables|Default|GetFirstIOSlot)) (Utilities|IsValid (Variables|Default|GetSecondIOSlot)))
    (bind _attachlocation (Class|InteractionInterface|QueryFactory(Message) (Variables|Default|GetFirstIOSlot)))
    (bind _attachlocation_2 (Class|InteractionInterface|QueryFactory(Message) (Variables|Default|GetSecondIOSlot)))
    (Spline|SetSplinePoints (Variables|Default|GetSpline) (Utilities|Array|MakeArray _attachlocation_2 _attachlocation) "World" true)
    (CallFunction|UpdateSplineMeshfromSpline)
    (CallFunction|SetupSocialDistancingArray)
    (bind _returnvalue (Utilities|Time|SetTimerbyEvent (delegate Custom|ProcessItems) (Variables|Default|GetTickSpeed) true))
    (Variables|Default|SetPullTimer _returnvalue)
    (else
      (Development|PrintString "PipeCastError"))))

(fn ConstructionScript)

(fn UpdateSplineMeshfromSpline
  (bind _spline (Variables|Default|GetSpline))
  (for _index (range 0 (- (Spline|GetNumberOfSplinePoints (Variables|Default|GetSpline)) 2))
    (bind _returnvalue (AddComponent|AddSplineMeshComponent true))
    (LocalVariables|SetTempSplineMesh _returnvalue)
    (Collision|SetCollisionProfileName (LocalVariables|GetTempSplineMesh) "BlockAll" true :!class /Script/Engine.PrimitiveComponent)
    (Transformation|SetMobility (LocalVariables|GetTempSplineMesh) "Movable")
    (Transformation|AttachComponentToComponent (LocalVariables|GetTempSplineMesh) (Variables|Default|GetDefaultSceneRoot) "None" "KeepRelative" "KeepRelative" "KeepRelative" true)
    (Components|StaticMesh|SetStaticMesh (LocalVariables|GetTempSplineMesh) "/Game/Models/PipeCylinder.PipeCylinder")
    (Rendering|Material|SetMaterial (LocalVariables|GetTempSplineMesh) 0 (LocalVariables|GetNewLocalVar_0))
    (SplineMesh|SetStartandEnd (LocalVariables|GetTempSplineMesh) (.Location (Spline|GetLocationandTangentatSplinePoint _spline _index "Local")) (.Tangent (Spline|GetLocationandTangentatSplinePoint _spline _index "Local")) (.Location (Spline|GetLocationandTangentatSplinePoint _spline (+ _index 1) "Local")) (.Tangent (Spline|GetLocationandTangentatSplinePoint _spline (+ _index 1) "Local")) true :!class /Script/Engine.SplineMeshComponent)))

(fn SetupSocialDistancingArray
  (bind _socialdistancing (Variables|Default|GetSocialDistancing))
  (bind _spline (Variables|Default|GetSpline))
  (bind _returnvalue (Spline|GetSplineLength _spline))
  (bind _returnvalue_2 (/ _returnvalue _socialdistancing))
  (bind _returnvalue_3 (Math|Float|Floor _returnvalue_2))
  (Utilities|Array|Resize (Variables|Default|GetItems) _returnvalue_3)
  (Utilities|Array|Resize (Variables|Default|GetItemHISMCIndexes) _returnvalue_3)
  (Utilities|Array|Resize (Variables|Default|GetHISMCTracker) _returnvalue_3)
  (for (_ _array_index) (Variables|Default|GetItemHISMCIndexes)
    (Utilities|Array|SetArrayElem (Variables|Default|GetItemHISMCIndexes) _array_index -1)))

(fn PushItemsThroughArray
  (bind _itemhismcindexes (Variables|Default|GetItemHISMCIndexes))
  (bind _items (Variables|Default|GetItems))
  (bind _hismctracker (Variables|Default|GetHISMCTracker))
  (bind _itemhismcindexes_2 (Variables|Default|GetItemHISMCIndexes))
  (bind _returnvalue (Utilities|Array|Length _items))
  (bind _returnvalue_2 (- _returnvalue 1))
  (for _index (range 0 _returnvalue_2)
    (if (== _returnvalue_2 (- _returnvalue_2 _index))
      (if (!= (Utilities|Array|Get(acopy) (Variables|Default|GetItemHISMCIndexes) _returnvalue_2) -1)
        (bind _hismc_index (CallFunction|FindHISMCforItem (Utilities|Array|Get(acopy) (Variables|Default|GetItems) (- _returnvalue_2 _index))))
        (Class|InstancedStaticMeshComponent|RemoveInstance (Utilities|Array|Get(acopy) (Variables|Default|GetItemHISMC) _hismc_index) (Utilities|Array|Get(acopy) (Variables|Default|GetItemHISMCIndexes) (- _returnvalue_2 _index)))
        (CallFunction|Subtract1fromHISMC (Utilities|Array|Get(acopy) (Variables|Default|GetItemHISMC) _hismc_index))
        (Utilities|Array|SetArrayElem (Variables|Default|GetItemHISMCIndexes) (- _returnvalue_2 _index) -1))
      (elif (and (== (- _returnvalue_2 _index) 0) (== (Utilities|Array|Get(acopy) (Variables|Default|GetItemHISMCIndexes) (+ (- _returnvalue_2 _index) 1)) -1))
        (Utilities|FlowControl|Sequence
          (:then_0
            (if (and (!= (Utilities|Array|Get(acopy) _itemhismcindexes_2 (- _returnvalue_2 _index)) -1) (== (Utilities|Array|Get(acopy) _itemhismcindexes_2 (+ (- _returnvalue_2 _index) 1)) -1)) :!label _label
              (bind _hismc_index_2 (CallFunction|FindHISMCforItem (Utilities|Array|Get(acopy) (Variables|Default|GetItems) (- _returnvalue_2 _index))))
              (Components|InstancedStaticMesh|UpdateInstanceTransform (Utilities|Array|Get(acopy) (Variables|Default|GetItemHISMC) _hismc_index_2) (Utilities|Array|Get(acopy) (Variables|Default|GetItemHISMCIndexes) (- _returnvalue_2 _index)) (Math|Transform|MakeTransform (Spline|GetLocationatDistanceAlongSpline (Variables|Default|GetSpline) (* (- 1.0 (/ (Math|Conversions|ToFloat(Integer) (- _returnvalue_2 _index)) (Math|Conversions|ToFloat(Integer) (- (Utilities|Array|Length (Variables|Default|GetItems)) 1)))) (Spline|GetSplineLength (Variables|Default|GetSpline))) "Local") "0, 0, 0" "0.050000,0.050000,0.050000") false false false)
              (Utilities|Array|SetArrayElem _itemhismcindexes (+ (- _returnvalue_2 _index) 1) (Utilities|Array|Get(acopy) (Variables|Default|GetItemHISMCIndexes) (- _returnvalue_2 _index)))
              (Utilities|Array|SetArrayElem _itemhismcindexes (- _returnvalue_2 _index) -1)
              (Utilities|Array|SetArrayElem _hismctracker (+ (- _returnvalue_2 _index) 1) (Utilities|Array|Get(acopy) _hismctracker (- _returnvalue_2 _index)))
              (Utilities|Array|SetArrayElem _hismctracker (- _returnvalue_2 _index) 0)))
          (:then_1
            (bind (_success_ _itempulled) (Class|InteractionInterface|GrabItemfromOutput(Message) (select (Variables|Default|GetFirstIsInput) (Variables|Default|GetFirstIOSlot) (Variables|Default|GetSecondIOSlot))))
            (if _success_
              (bind _hismc_index_3 (CallFunction|FindHISMCforItem _itempulled))
              (bind _returnvalue_3 (Components|InstancedStaticMesh|AddInstance (Utilities|Array|Get(acopy) (Variables|Default|GetItemHISMC) _hismc_index_3) (Math|Transform|MakeTransform (Spline|GetLocationatDistanceAlongSpline (Variables|Default|GetSpline) (Spline|GetSplineLength (Variables|Default|GetSpline)) "Local") "0, 0, 0" "0.050000,0.050000,0.050000")))
              (Utilities|Array|SetArrayElem (Variables|Default|GetItemHISMCIndexes) 0 _returnvalue_3)
              (Utilities|Array|SetArrayElem (Variables|Default|GetHISMCTracker) 0 (Utilities|Array|Get(acopy) (Variables|Default|GetItemHISMC) _hismc_index_3)))))
        (else
          (goto _label))))))

(fn FindHISMCforItem
  (params (Item :type E_ItemTypes%20Enum :default "NewEnumerator0"))
  (bind (_valid_ _data) (CallFunction|GetItemDatafromEnum Item))
  (if _valid_
    (LocalVariables|SetTempItemStore _data)
    (for (_array_element _array_index) (Variables|Default|GetItemHISMC)
      (if (and (== (.model (LocalVariables|GetTempItemStore)) (Variables|/Script/Engine.StaticMeshComponent|GetStaticMesh _array_element)) (== (.material (LocalVariables|GetTempItemStore)) (Rendering|Material|GetMaterial _array_element 0)))
        (return _array_index)))
    (bind _returnvalue (AddComponent|AddHierarchicalInstancedStaticMeshComponent false))
    (Components|StaticMesh|SetStaticMesh _returnvalue (.model (LocalVariables|GetTempItemStore)))
    (Rendering|Material|SetMaterial _returnvalue 0 (.material (LocalVariables|GetTempItemStore)))
    (bind _returnvalue_2 (Utilities|Array|Add (Variables|Default|GetItemHISMC) _returnvalue))
    (return _returnvalue_2)
    (else
      (Development|PrintString "Invalid Item")
      (return -1))))

(fn Subtract1fromHISMC
  (params (InputHISMC :type Hierarchical%20Instanced%20Static%20Mesh%20Component%20Object%20Reference))
  (bind _itemhismcindexes (Variables|Default|GetItemHISMCIndexes))
  (for (_array_element _array_index) (Variables|Default|GetHISMCTracker)
    (if (== _array_element InputHISMC)
      (Utilities|Array|SetArrayElem _itemhismcindexes _array_index (- (Utilities|Array|Get(acopy) _itemhismcindexes _array_index) 1))
      (Development|PrintString "Hello"))))