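; BPL_ItemLibrary is a function library that looks up item definitions in the DT_Items data table.
; GetItemFromResourceType maps a resource to a row and returns an item slot with the given stack size; GetItemDataFromEnum returns row data for an item enum.
; Both switch on hardcoded row names and report validity.
; The names are mismatched: Coal gets CopperOre, Copper gets IronOre, and every enum case reads CopperOre.
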(fn GetItemfromResourceType
  (params (Resource :type E_ResourceTypes%20Enum :default "NewEnumerator0") (CurrentStackOverride :type Integer))
  (switch Utilities|FlowControl|Switch|SwitchonE_ResourceTypes Resource
    (:NewEnumerator0
      (bind _returnvalue (Utilities|GetDataTableRow "/Game/Blueprints/Data/DT/DT_Items.DT_Items" "CopperOre")
        (:then
          (LocalVariables|SetItemType _returnvalue)
          (return true (Utilities|Struct|MakeS_ItemSlot (LocalVariables|GetItemType) CurrentStackOverride)))
        (:RowNotFound
          _)))
    (:NewEnumerator1
      (bind _returnvalue_2 (Utilities|GetDataTableRow "/Game/Blueprints/Data/DT/DT_Items.DT_Items" "IronOre")
        (:then
          (LocalVariables|SetItemType _returnvalue_2)
          (return true (Utilities|Struct|MakeS_ItemSlot (LocalVariables|GetItemType) CurrentStackOverride)))
        (:RowNotFound
          _)))
    (:NewEnumerator2
      (bind _returnvalue_3 (Utilities|GetDataTableRow "/Game/Blueprints/Data/DT/DT_Items.DT_Items" "IronOre")
        (:then
          (LocalVariables|SetItemType _returnvalue_3)
          (return true (Utilities|Struct|MakeS_ItemSlot (LocalVariables|GetItemType) CurrentStackOverride)))
        (:RowNotFound
          _))))
  (return false ""))

(fn GetItemDatafromEnum
  (params (Input :type E_ItemTypes%20Enum :default "NewEnumerator0"))
  (switch Utilities|FlowControl|Switch|SwitchonE_ItemTypes Input
    (:NewEnumerator0
      (bind _returnvalue (Utilities|GetDataTableRow "/Game/Blueprints/Data/DT/DT_Items.DT_Items" "CopperOre")
        (:then
          (LocalVariables|SetOutput _returnvalue)
          (return true (LocalVariables|GetOutput)))
        (:RowNotFound
          _)))
    (:NewEnumerator1
      (bind _returnvalue_2 (Utilities|GetDataTableRow "/Game/Blueprints/Data/DT/DT_Items.DT_Items" "CopperOre")
        (:then
          (LocalVariables|SetOutput _returnvalue_2)
          (return true (LocalVariables|GetOutput)))
        (:RowNotFound
          _)))
    (:NewEnumerator2
      (bind _returnvalue_3 (Utilities|GetDataTableRow "/Game/Blueprints/Data/DT/DT_Items.DT_Items" "CopperOre")
        (:then
          (LocalVariables|SetOutput _returnvalue_3)
          (return true (LocalVariables|GetOutput)))
        (:RowNotFound
          _))))
  (return false ""))