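; BP_ResourceNode is a world resource deposit that a single miner can attach to.
; AttachMiner flags the node as occupied, shrinks its Box to a minimal extent without updating overlaps, and returns the AttachLocation world position and resource type.
; QueryResourceNode reports occupancy and type, while QueryFactory returns invalid, so query callers can tell it apart from a factory.
; The event graph and construction script are empty.
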(event EventBeginPlay)

(event Collision|EventActorBeginOverlap
  (params (OtherActor :type Actor%20Object%20Reference)))

(event EventTick
  (params (DeltaSeconds :type Float%20%28single-precision%29)))

(fn ConstructionScript)

(fn AttachMiner
  (Variables|Default|SetMinerAttached? true)
  (Components|Box|SetBoxExtent (Variables|Default|GetBox) "1.000000,1.000000,1.000000" false)
  (return (Transformation|GetWorldLocation (Variables|Default|GetAttachLocation)) (Variables|Default|GetResourceType)))

(fn QueryFactory
  (return false "NewEnumerator0" "0, 0, 0"))

(fn QueryResourceNode
  (return true (Variables|Default|GetMinerAttached?) (Variables|Default|GetResourceType)))